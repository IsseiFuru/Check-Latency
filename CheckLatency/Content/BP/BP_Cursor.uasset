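; BP_Cursor is an actor that mirrors the cursor data held in the game instance.
; Each tick it compares OneCursor's position with BeforeCursor's and, when they differ, copies OneCursor into BeforeCursor and switches on its state.
; Update converts the measured value to a vector and moves the actor there, while Remove destroys it after a short delay.
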(event EventTick
  (params (DeltaSeconds :type Float%20%28single-precision%29))
  (bind _asclgame_instance (CallFunction|GetGameInstanceRef))
  (if (Utilities|Operators|NotEqual(!=) (.Position (Utilities|Struct|BreakF_Cursor (Variables|/Game/BP/CLGameInstance.CLGameInstance_C|GetOneCursor _asclgame_instance))) (.position (Variables|/Game/BP/CLGameInstance.CLGameInstance_C|GetBeforeCursor _asclgame_instance)) 0.0)
    (Variables|/Game/BP/CLGameInstance.CLGameInstance_C|SetBeforeCursor _asclgame_instance (Variables|/Game/BP/CLGameInstance.CLGameInstance_C|GetOneCursor _asclgame_instance))
    (switch string (.State (Utilities|Struct|BreakF_Cursor (Variables|/Game/BP/CLGameInstance.CLGameInstance_C|GetOneCursor _asclgame_instance)))
      (:update
        ;[0.01 0.35 1] code : update
        (bind _vector (CallFunction|FromMeasuredValuetoVector (.Position (Utilities|Struct|BreakF_Cursor (Variables|/Game/BP/CLGameInstance.CLGameInstance_C|GetOneCursor _asclgame_instance)))))
        (Transformation|SetActorLocation _vector false false))
      (:remove
        ;[0.01 0.35 1] code : remove
        (Utilities|FlowControl|Delay 0.1)
        (Actor|DestroyActor)))))

(fn ConstructionScript)